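; BP_Sandwich is a sandwich actor whose ingredient components are revealed by name.
; Showingredient converts the given name and switches on it, making the matching group of components visible: Bread, Ham, Olive with Paprika, Onion or Tomato.
; Any unmatched name falls through to the default, which shows both the mustard and white sauce components.
; It only turns visibility on; the event graph and construction script hold no logic.
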(fn `Showingredient`
  (params (IngredientName :type String))
  (switch `name` (`KismetStringLibrary.Conv_StringToName` IngredientName)
    (:`Default`
      (`SceneComponent.SetVisibility` (`self.Mustard1`) true false)
      (`SceneComponent.SetVisibility` (`self.Mustard`) true false)
      (`SceneComponent.SetVisibility` (`self.WhiteSource`) true false)
      (`SceneComponent.SetVisibility` (`self.WhiteSource1`) true false))
    (:`Bread`
      (`SceneComponent.SetVisibility` (`self.Bread`) true false))
    (:`Ham`
      (`SceneComponent.SetVisibility` (`self.Ham`) true false)
      (`SceneComponent.SetVisibility` (`self.Ham1`) true false)
      (`SceneComponent.SetVisibility` (`self.Ham2`) true false))
    (:`Olive`
      (`SceneComponent.SetVisibility` (`self.Olive`) true false)
      (`SceneComponent.SetVisibility` (`self.Olive1`) true false)
      (`SceneComponent.SetVisibility` (`self.Olive2`) true false)
      (`SceneComponent.SetVisibility` (`self.paprika`) true false)
      (`SceneComponent.SetVisibility` (`self.paprika1`) true false)
      (`SceneComponent.SetVisibility` (`self.paprika2`) true false))
    (:`Onion`
      (`SceneComponent.SetVisibility` (`self.Onion`) true false)
      (`SceneComponent.SetVisibility` (`self.Onion2`) true false)
      (`SceneComponent.SetVisibility` (`self.Onion3`) true false))
    (:`Tomato`
      (`SceneComponent.SetVisibility` (`self.Tomato`) true false)
      (`SceneComponent.SetVisibility` (`self.Tomato2`) true false))))

(fn `UserConstructionScript`)