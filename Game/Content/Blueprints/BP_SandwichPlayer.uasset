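; Player-side actor that carries a sandwich and builds it up from dishes that enter its drop zone.
; On BeginPlay it spawns a scaled-down BP_Sandwich from the Location component's relative transform, then snaps it to that component's world location every Tick.
; When a BP_Dish overlaps DropZone, it shows that dish's ingredient on the sandwich and destroys the dish.
; Unconnected per-ingredient calls and a DestroyActor node never run.
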(event `self.ReceiveBeginPlay`
  (bind (_returnvalue_location _returnvalue_rotation) (`KismetMathLibrary.BreakTransform` (`SceneComponent.GetRelativeTransform` (`self.Location`))))
  (bind _returnvalue (`|SpawnActorFromClass` "/Game/Blueprints/BP_Sandwich.BP_Sandwich_C" (`KismetMathLibrary.MakeTransform` _returnvalue_location _returnvalue_rotation (0.2 0.2 0.2)) "Undefined" "MultiplyWithRoot" null null))
  (bind _output_get (set `self.Sandwich` _returnvalue))
  (set `self.MySandwich` _output_get))

(event `self.ReceiveTick`
  (params (DeltaSeconds :type "Float (single-precision)"))
  (`self.K2_SetActorLocation` (`self.Sandwich`) (`SceneComponent.K2_GetComponentLocation` (`self.Location`)) false false))

(event `self.DropZone.OnComponentBeginOverlap`
  (params (OverlappedComponent :type "PrimitiveComponent Object Reference") (OtherActor :type "Actor Object Reference") (OtherComp :type "PrimitiveComponent Object Reference") (OtherBodyIndex :type Integer) (bFromSweep :type Boolean) (SweepResult :type "HitResult Structure (by ref)"))
  (bind _asbp_dish (cast `/Game/Models/Food/BP_Dish` OtherActor))
  (`/Game/Blueprints/BP_Sandwich.Showingredient` (`self.MySandwich`) (`/Game/Models/Food/BP_Dish.MyIngredient` _asbp_dish))
  (`self.K2_DestroyActor` _asbp_dish))

(fn `UserConstructionScript`)